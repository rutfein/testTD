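; Player controller for a top-down pan camera that drives the cameraPawn through movement, zoom and screen-edge scrolling.
; Axis inputs pan along the pawn's local axes, scaled by zoom distance and a Shift boost, while a macro turns mouse position at viewport edges into scroll offsets.
; Zoom inputs set clamped arm-length and pitch goals together, which Tick eases toward with FInterpTo.
; DisableCamNav blocks panning and edge scrolling, but not zoom.
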(event `self.ReceiveBeginPlay`
  (`|ExecutionSequence`
    (:`then_0`
      (`self.referenceCasts`))))

(event `self.ReceiveTick`
  (params (DeltaSeconds :type "Float (single-precision)"))
  (bind _sphere (`/Game/rutrug/camera/blueprints/cameraPawn.Sphere` (`self.cameraPanRef`)))
  ;[1 1 1] Tick
  (set `self.delta` DeltaSeconds)
  (`|ExecutionSequence`
    (:`then_0`
      (if (not (`KismetMathLibrary.NearlyEqual_FloatFloat` (`self.cameraGoal`) (`SpringArmComponent.TargetArmLength` (`/Game/rutrug/camera/blueprints/cameraPawn.SpringArm` (`self.cameraPanRef`))) 0.1))
        (bind _distance (`self.calcCameraDistance`))
        (set `SpringArmComponent.TargetArmLength` _distance (`/Game/rutrug/camera/blueprints/cameraPawn.SpringArm` (`self.cameraPanRef`)))))
    (:`then_1`
      (if (not (`KismetMathLibrary.NearlyEqual_FloatFloat` (`self.tiltGoal`) (.pitch (`SceneComponent.K2_GetComponentRotation` (`/Game/rutrug/camera/blueprints/cameraPawn.Sphere` (`self.cameraPanRef`)))) 0.01))
        (bind _distance_2 (`self.calcTiltDistance`)
          (:`execute2`
            (`SceneComponent.K2_SetWorldRotation` _sphere (`KismetMathLibrary.MakeRotator` (.roll (`SceneComponent.K2_GetComponentRotation` _sphere)) _distance_2 (.yaw (`SceneComponent.K2_GetComponentRotation` _sphere))) false false)))))))

(event `InputAxis|moveForward`
  (params (AxisValue :type "Float (single-precision)"))
  ;[1 1 1] MovementX
  (if (not (`self.disableCamNav`))
    (`self.K2_SetActorTransform` (`self.cameraPanRef`) (`self.movementX` (`self.movementSpeedCalculation`) (`self.fastMoveMultiplier`) AxisValue (`self.cameraPanRef`)) false false)))

(event `InputAction|zoomIn`
  (params (Key :type "Key Structure" :default "AnyKey"))
  ;[1 1 1] Zoom camera distance
  (:`Pressed`
    (set `self.cameraGoal` (`KismetMathLibrary.FClamp` (- (`SpringArmComponent.TargetArmLength` (`/Game/rutrug/camera/blueprints/cameraPawn.SpringArm` (`self.cameraPanRef`))) (`self.zoomSensitivity`)) 500.0 (`self.maxArmDistance`)))))

(event `InputAction|zoomOut`
  (params (Key :type "Key Structure" :default "AnyKey"))
  ;[1 1 1] Zoom camera distance
  (:`Pressed`
    (set `self.cameraGoal` (`KismetMathLibrary.FClamp` (+ (`SpringArmComponent.TargetArmLength` (`/Game/rutrug/camera/blueprints/cameraPawn.SpringArm` (`self.cameraPanRef`))) (`self.zoomSensitivity`)) 500.0 (`self.maxArmDistance`)))))

(event `InputAxis|moveRight`
  (params (AxisValue :type "Float (single-precision)"))
  ;[1 1 1] MovementY
  (if (not (`self.disableCamNav`))
    (`self.K2_SetActorTransform` (`self.cameraPanRef`) (`self.movementY` AxisValue (`self.movementSpeedCalculation`) (`self.fastMoveMultiplier`) (`self.cameraPanRef`)) false false)))

(event `InputAxisKey|MouseX`
  (params (AxisValue :type "Float (single-precision)"))
  ;[1 1 1] Edge movement
  (if (not (`self.disableCamNav`))
    (bind (_deltayspeed _deltaxspeed) (`self.screenEdgeMovement` :!label _label))
    (`self.K2_AddActorLocalOffset` (`self.cameraPanRef`) (`KismetMathLibrary.MakeVector` _deltaxspeed _deltayspeed) true false)))

(event `InputAction|zoomIn`
  (params (Key :type "Key Structure" :default "AnyKey"))
  ;[1 1 1] Zoom camera tilt
  (:`Pressed`
    (set `self.tiltGoal` (`KismetMathLibrary.FClamp` (+ (.pitch (`SceneComponent.K2_GetComponentRotation` (`/Game/rutrug/camera/blueprints/cameraPawn.Sphere` (`self.cameraPanRef`)))) (`self.tiltSensitivity`)) -75.0 -45.0))))

(event `InputAxisKey|MouseY`
  (params (AxisValue :type "Float (single-precision)"))
  ;[1 1 1] Edge movement
  (if (not (`self.disableCamNav`))
    (goto _label :!via `mouseY`)))

(event `Key|LeftShift`
  (params (Key :type "Key Structure" :default "AnyKey"))
  ;[1 1 1] Shift speed multiplier
  (:`Pressed`
    (set `self.fastMoveMultiplier` 2.0))
  (:`Released`
    (set `self.fastMoveMultiplier` 1.0)))

(event `InputAction|zoomOut`
  (params (Key :type "Key Structure" :default "AnyKey"))
  ;[1 1 1] Zoom camera tilt
  (:`Pressed`
    (set `self.tiltGoal` (`KismetMathLibrary.FClamp` (- (.pitch (`SceneComponent.K2_GetComponentRotation` (`/Game/rutrug/camera/blueprints/cameraPawn.Sphere` (`self.cameraPanRef`)))) (`self.tiltSensitivity`)) -75.0 -45.0))))

(fn `movementSpeedCalculation`
  (returns (moveSensitivity :type "Float (double-precision)"))
  (return (`KismetMathLibrary.FClamp` (/ (`SpringArmComponent.TargetArmLength` (`/Game/rutrug/camera/blueprints/cameraPawn.SpringArm` (`self.cameraPanRef`))) 100.0) 5.0 20.0)))

(fn `UserConstructionScript`)